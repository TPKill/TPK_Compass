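; Mod controller for the TPK Compass mod that supplies clients with clanmate positions and merges its UI module data table.
; On dedicated servers, looping timers rebuild replicated maps of guild members and guilded players' rounded XY positions, skipping players inside dungeons.
; Values are packed as comma-separated strings.
; Client OnRep handlers unpack them into MyClan and MyClanPos, keeping only the local player's guildmates.
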(event `self.ReceiveBeginPlay`
  (if (`KismetSystemLibrary.IsDedicatedServer`)
    (`KismetSystemLibrary.K2_SetTimer` null "UpdateRepGuildMap" 15.0 true)
    (`KismetSystemLibrary.K2_SetTimer` null "UpdateRepPawnPos" 5.0 true)
    (else
      (`self.SetMyClan`))))

(fn `AddValue`
  (params (MapArray :type "Map of String to String") (Key :type String) (Value :type String))
  (returns (RetMap :type "Map of String to String") (Dirty :type Boolean))
  (locals (retDirty :type Boolean) (Arr :type "Array of String"))
  (bind (_value _returnvalue) (`BlueprintMapLibrary.Map_Find` MapArray Key))
  (if _returnvalue
    (bind _output_get (set `local.Arr` (`KismetStringLibrary.ParseIntoArray` _value ",")))
    (if (not (`KismetArrayLibrary.Array_Contains` _output_get Value))
      (`KismetArrayLibrary.Array_Add` _output_get Value)
      (`BlueprintMapLibrary.Map_Add` MapArray Key (`KismetStringLibrary.JoinStringArray` _output_get ","))
      (set `local.retDirty` true))
    (else
      (`BlueprintMapLibrary.Map_Add` MapArray Key Value)
      (set `local.retDirty` true)))
  (return MapArray (`local.retDirty`)))

(fn `ModDataTableOperations`
  (`self.MergeDataTables` "/Game/UI/UIModuleTable.UIModuleTable" "/Game/Mods/TPK_Compass/UI/d_TPK_Compass_UIModuleTable.d_TPK_Compass_UIModuleTable"))

(fn `OnRep_RepGuildMap`
  (`self.SetMyClan`)
  (return))

(fn `OnRep_RepPawnPos`
  (locals (ClanPos :type "Map of Integer to Vector Structure") (MyID :type String))
  (if (`KismetSystemLibrary.IsDedicatedServer`)
    (return)
    (else
      (set `local.MyID` (`KismetStringLibrary.Conv_IntToString` (`PlayerState.PlayerId` (`Controller.PlayerState` (`GameplayStatics.GetPlayerController` 0)))))
      (for _array_element (`self.MyClan`)
        (bind _returnvalue (`KismetStringLibrary.Conv_IntToString` _array_element))
        (bind (_value _returnvalue_2) (`BlueprintMapLibrary.Map_Find` (`.Map` (break `ReplicatedTMap` (`self.RepPawnPos`))) _returnvalue))
        (`/Game/Systems/BP_MacroGlobal.And+Branch` _returnvalue_2 (`KismetStringLibrary.NotEqual_StrStr` _returnvalue (`local.MyID`))
          (:`True`
            (bind _returnvalue_3 (`KismetStringLibrary.ParseIntoArray` _value ","))
            (`BlueprintMapLibrary.Map_Add` (`local.ClanPos`) _array_element (`KismetMathLibrary.MakeVector` (`KismetStringLibrary.Conv_StringToDouble` (`KismetArrayLibrary.Array_Get` _returnvalue_3)) (`KismetStringLibrary.Conv_StringToDouble` (`KismetArrayLibrary.Array_Get` _returnvalue_3 1)))))))
      (set `self.MyClanPos` (`local.ClanPos`))
      (return))))

(fn `RemoveValue`
  (params (MapArray :type "Map of String to String") (Key :type String) (Value :type String))
  (returns (ReturnMapArray :type "Map of String to String"))
  (locals (Arr :type "Array of String"))
  (bind (_value _returnvalue) (`BlueprintMapLibrary.Map_Find` MapArray Key))
  (if _returnvalue
    (bind _output_get (set `local.Arr` (`KismetStringLibrary.ParseIntoArray` _value ",")))
    (`KismetArrayLibrary.Array_RemoveItem` _output_get Value)
    (`BlueprintMapLibrary.Map_Add` MapArray Key (`KismetStringLibrary.JoinStringArray` (`local.Arr`) ",")))
  (return MapArray))

(fn `SetMyClan`
  (locals (TmpIntArr :type "Array of Integer") (TmpStrArr :type "Array of String"))
  (bind _returnvalue (`GameplayStatics.GetPlayerController` 0))
  (bind _tmpintarr (`local.TmpIntArr`))
  (bind _returnvalue_2 (`ConanCharacter.GetGuild` (cast `/Game/Characters/BaseBPCombat` (`Controller.K2_GetPawn` _returnvalue) :!pure true)))
  (if (`KismetSystemLibrary.IsDedicatedServer`)
    (return)
    (else
      (`/Engine/EditorBlueprintResources/StandardMacros.IsValid` _returnvalue_2
        (:`Is Valid`
          (bind _output_get (set `local.TmpStrArr` (`KismetStringLibrary.ParseIntoArray` (`BlueprintMapLibrary.Map_Find` (`.Map` (break `ReplicatedTMap` (`self.RepGuildMap`))) (`Guild.GetGuildName` _returnvalue_2)) ",")))
          (`KismetArrayLibrary.Array_RemoveItem` _output_get (`KismetStringLibrary.Conv_IntToString` (`PlayerState.PlayerId` (`Controller.PlayerState` _returnvalue))))
          (for _array_element _output_get
            (`KismetArrayLibrary.Array_Add` _tmpintarr (`KismetStringLibrary.Conv_StringToInt` _array_element)))
          (set `self.MyClan` _tmpintarr)
          (return))
        (:`Is Not Valid`
          (`KismetArrayLibrary.Array_Clear` (`self.MyClan`))
          (return))))))

(fn `UpdateRepGuildMap`
  (locals (TempSet :type "Map of String to String") (TempMembers :type "Array of String") (CompareSet :type "Map of String to String"))
  (bind _tempset (`local.TempSet`))
  (bind _output_get (set `local.TempSet` (`.Map` (break `ReplicatedTMap` (`self.RepGuildMap`)))))
  (set `local.CompareSet` _output_get)
  (bind _outactors (`GameplayStatics.GetAllActorsOfClass` "/Script/ConanSandbox.ConanPlayerController"))
  (for _array_element _outactors
    (bind _returnvalue (`ConanPlayerController.GetConanCharacter` _array_element))
    (bind _returnvalue_2 (`ConanCharacter.GetGuild` _returnvalue))
    (if (`KismetSystemLibrary.IsValid` _returnvalue_2)
      (bind _returnvalue_3 (`Guild.GetGuildName` _returnvalue_2))
      (bind _returnvalue_4 (`KismetStringLibrary.Conv_IntToString` (`PlayerState.PlayerId` (`Pawn.PlayerState` _returnvalue))))
      (bind _retmap (`self.AddValue` (`local.TempSet`) _returnvalue_3 _returnvalue_4))
      (set `local.TempSet` _retmap)
      (bind _returnmaparray (`self.RemoveValue` (`local.CompareSet`) _returnvalue_3 _returnvalue_4))
      (set `local.CompareSet` _returnmaparray)))
  ;[1 1 1] Clear left users
  (bind _keys (`BlueprintMapLibrary.Map_Keys` (`local.CompareSet`)))
  (for _array_element_2 _keys
    (for _array_element_3 (`KismetStringLibrary.ParseIntoArray` (`BlueprintMapLibrary.Map_Find` (`local.CompareSet`) _array_element_2) ",")
      (bind _returnmaparray_2 (`self.RemoveValue` (`local.TempSet`) _array_element_2 _array_element_3))
      (set `local.TempSet` _returnmaparray_2)))
  ;[1 1 1] Clear empty clans
  (bind _keys_2 (`BlueprintMapLibrary.Map_Keys` _tempset))
  (for _array_element_4 _keys_2
    (if (not (> (`KismetStringLibrary.Len` (`BlueprintMapLibrary.Map_Find` _tempset _array_element_4)) 0))
      (`BlueprintMapLibrary.Map_Remove` _tempset _array_element_4)))
  ;[1 1 1] Push
  (set `self.RepGuildMap` (make `ReplicatedTMap` (`local.TempSet`)))
  (return))

(fn `UpdateRepPawnPos`
  (locals (PosMap :type "Map of String to String"))
  (bind _posmap (`local.PosMap`))
  (`BlueprintMapLibrary.Map_Clear` _posmap)
  (bind _outactors (`GameplayStatics.GetAllActorsOfClass` "/Script/ConanSandbox.ConanPlayerController"))
  (for _array_element _outactors
    (bind _returnvalue (`ConanPlayerController.GetConanCharacter` _array_element))
    (bind _feetlocation (`/Game/Characters/FuncomFunctionLibrary.GetActorFeetLocation` _returnvalue))
    (if (`FuncomGenericLibrary.IsLocationInsideDungeon` _returnvalue _feetlocation)
      _
      (elif (`KismetSystemLibrary.IsValid` (`ConanCharacter.GetGuild` _returnvalue))
        (`BlueprintMapLibrary.Map_Add` (`local.PosMap`) (`KismetStringLibrary.Conv_IntToString` (`PlayerState.PlayerId` (`Pawn.PlayerState` _returnvalue))) (`KismetStringLibrary.Concat_StrStr` (`KismetStringLibrary.Conv_IntToString` (`KismetMathLibrary.Round` (.x _feetlocation))) "," (`KismetStringLibrary.Conv_IntToString` (`KismetMathLibrary.Round` (.y _feetlocation))))))))
  (set `self.RepPawnPos` (make `ReplicatedTMap` _posmap))
  (return))

(fn `UserConstructionScript`)